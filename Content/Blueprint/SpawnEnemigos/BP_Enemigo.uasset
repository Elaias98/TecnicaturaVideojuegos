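; BP_Enemigo is an enemy actor that randomly decides on BeginPlay whether it moves.
; While moving, each Tick offsets it locally by Speed without sweep, calls QuitarVida with zero and prints Life on screen.
; QuitarVida sets Life to its input minus Life, so that zero input flips Life's sign every frame.
; Stationary enemies only print a debug message each Tick.
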(event `self.ReceiveBeginPlay`
  (set `self.bSeMueve` (`KismetMathLibrary.RandomBool`)))

(event `self.ReceiveTick`
  (params (DeltaSeconds :type "Float (single-precision)"))
  (if (`self.bSeMueve`)
    (`self.K2_AddActorLocalOffset` (`self.speed`))
    (`self.QuitarVida` 0.0)
    (`KismetSystemLibrary.PrintString` (`KismetStringLibrary.Conv_DoubleToString` (`self.life`)) true true (struct :`G` 1.0 :`B` 0.043339 :`A` 1.0) 5000.0 "2")
    (else
      (`KismetSystemLibrary.PrintString` "No se Movio" true true (struct :`R` 1.0 :`A` 1.0) 3.0 "2"))))

(fn `QuitarVida`
  (params (`10` :type "Float (double-precision)"))
  (set `self.life` (- `10` (`self.life`))))

(fn `UserConstructionScript`)