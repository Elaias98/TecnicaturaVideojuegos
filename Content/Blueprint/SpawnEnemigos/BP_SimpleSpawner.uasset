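; BP_SimpleSpawner is an actor that spawns enemies on a repeating timer.
; From BeginPlay, a looping three-second timer fires the Spawner event, which spawns a BP_Enemigo at the spawner's transform with its Speed and Life values.
; A separate QuitarVida function, not called in this graph, sets Life to its input minus current Life and prints the result on screen.
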(event `self.ReceiveBeginPlay`
  (`KismetSystemLibrary.K2_SetTimerDelegate` (delegate `Spawner`) 3.0 true))

(event `Spawner`
  (`|SpawnActorFromClass` "/Game/Blueprint/SpawnEnemigos/BP_Enemigo.BP_Enemigo_C" (`self.GetTransform`) "Undefined" "MultiplyWithRoot" null (`self.speed`) (`self.life`) null))

(fn `QuitarVida`
  (params (`10` :type "Float (double-precision)"))
  (bind _output_get (set `self.life` (- `10` (`self.life`))))
  (`KismetSystemLibrary.PrintString` (`KismetStringLibrary.Conv_DoubleToString` _output_get) true true (struct :`G` 1.0 :`B` 0.0325 :`A` 1.0) 100000.0 "2"))

(fn `UserConstructionScript`)