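; BP_Lvlup is a conditionals practice Blueprint that simulates gaining experience and levelling up.
; BeginPlay starts a looping 0.1-second timer on SubirNivel, which adds one Experiencia through SumarExperiencia and prints the total.
; Once Experiencia reaches the threshold of 100, every tick of the timer sets Nivel to 2 and prints it in green.
; The ClearTimerByFunctionName call after timer setup has an empty name, so the loop keeps running.
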(event `self.ReceiveTick`
  (params (DeltaSeconds :type "Float (single-precision)")))

(event `self.ReceiveBeginPlay`
  (`KismetSystemLibrary.K2_SetTimerDelegate` (delegate `SubirNivel`) 0.1 true)
  (`KismetSystemLibrary.K2_ClearTimer` null))

(event `SubirNivel`
  (bind _experiencia (`self.experiencia`))
  (`self.SumarExperiencia` 1)
  (`KismetSystemLibrary.PrintString` (`KismetStringLibrary.Conv_IntToString` _experiencia) true true (struct :`G` 0.66 :`B` 1.0 :`A` 1.0) 8000.0 "2")
  (if (>= _experiencia 100)
    (bind _output_get (set `self.nivel` 2))
    (`KismetSystemLibrary.PrintString` (`KismetStringLibrary.Conv_IntToString` _output_get) true true (struct :`R` 0.108294 :`G` 1.0 :`B` 0.218351 :`A` 1.0) 800000.0 "2")))

(fn `SumarExperiencia`
  (params (Exp :type Integer :default 1))
  (set `self.experiencia` (+ Exp (`self.experiencia`))))

(fn `UserConstructionScript`)